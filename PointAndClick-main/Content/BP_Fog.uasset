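; BP_Fog is a placeable fog actor that renders scrolling, masked fog through the material on its Cube mesh.
; Its Construction Script creates a dynamic instance of the cube's material and pushes the actor's mask, opacity, speed and color variables into it as parameters.
; The event graph is empty, so the Blueprint does no work on Tick or overlap.
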(event EventBeginPlay)

(event Collision|EventActorBeginOverlap
  (params (OtherActor :type Actor%20Object%20Reference)))

(event EventTick
  (params (DeltaSeconds :type Float%20%28single-precision%29)))

(fn ConstructionScript
  (bind _cube (Variables|Default|GetCube))
  (bind _returnvalue (Rendering|Material|CreateDynamicMaterialInstance _cube 0 (Rendering|Material|GetMaterial _cube 0) "" :!class /Script/Engine.PrimitiveComponent))
  (Variables|Default|SetMaterialDyna _returnvalue)
  (Utilities|FlowControl|Sequence
    (:then_0
      (Rendering|Material|SetScalarParameterValue (Variables|Default|GetMaterialDyna) "MaskSize" (Variables|Default|GetMaskSize) :!class /Script/Engine.MaterialInstanceDynamic))
    (:then_1
      (Rendering|Material|SetScalarParameterValue (Variables|Default|GetMaterialDyna) "Opacity" (Variables|Default|GetOpacity) :!class /Script/Engine.MaterialInstanceDynamic))
    (:then_2
      (Rendering|Material|SetScalarParameterValue (Variables|Default|GetMaterialDyna) "SpeedX" (Variables|Default|GetSpeedX) :!class /Script/Engine.MaterialInstanceDynamic))
    (:then_3
      (Rendering|Material|SetScalarParameterValue (Variables|Default|GetMaterialDyna) "SpeedY" (Variables|Default|GetSpeedY) :!class /Script/Engine.MaterialInstanceDynamic))
    (:then_4
      (Rendering|Material|SetVectorParameterValue (Variables|Default|GetMaterialDyna) "FogColor" (Variables|Default|GetFogColor) :!class /Script/Engine.MaterialInstanceDynamic))
    (:then_5
      (Rendering|Material|SetVectorParameterValue (Variables|Default|GetMaterialDyna) "MaskControls" (Variables|Default|GetMaskControls) :!class /Script/Engine.MaterialInstanceDynamic))))