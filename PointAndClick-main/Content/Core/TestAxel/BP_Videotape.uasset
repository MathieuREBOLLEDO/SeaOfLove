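; BP_Videotape is a collectible VHS tape actor identified by a videotape number.
; The construction script uses that number to pull its material and page name from the TapesID array.
; When destroyed or when its Acquired? event fires, it finds BP_TapeSelection in the level and reports the number through TapeAcquired.
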(event Custom|Acquired?
  (bind _returnvalue (Actor|GetActorOfClass "/Game/Core/TestAxel/BP_TapeSelection.BP_TapeSelection_C"))
  (Default|TapeAcquired _returnvalue (Variables|Default|GetVideotapeNumber)))

(event EventBeginPlay)

(event EventDestroyed
  (bind _returnvalue (Actor|GetActorOfClass "/Game/Core/TestAxel/BP_TapeSelection.BP_TapeSelection_C"))
  (Default|TapeAcquired _returnvalue (Variables|Default|GetVideotapeNumber)))

(fn ConstructionScript
  (bind _videotapenumber (Variables|Default|GetVideotapeNumber))
  (bind _tapesid (Variables|Default|GetTapesID))
  (bind _output (Utilities|Array|Get(acopy) _tapesid _videotapenumber))
  (Rendering|Material|SetMaterial (Variables|Default|GetStaticMesh) 0 (.vhs_material _output))
  (Variables|Default|SetVideotapeName (.page _output)))