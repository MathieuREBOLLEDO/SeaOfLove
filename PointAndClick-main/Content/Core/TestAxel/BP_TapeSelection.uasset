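; Work-in-progress VHS tape selection Blueprint that tracks acquired tapes as pages, with debug prints as its only output.
; TapeAcquired copies the TapesIDCopy entry at TapeID into the same TapesPossessed slot, then prints page numbers.
; Selection and BeginPlay are empty, leaving page stepping and the TapesIDCopy fill from BP_Videotape unconnected.
; LoopBas and LoopHaut wrap PageSelection using the array length, one past the last index.
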(event Custom|Selection
  (params (PageDirection :type Integer)))

(event Custom|TapeAcquired
  (params (Tape_ID :type Integer))
  ;[1 1 1] PRINT - VHS Acquired
  (Development|PrintString (Utilities|String|Append "VHS Acquired : " (Utilities|String|ToString(Name) "None") "  //  N°" (Utilities|String|ToString(Integer) (.pagenumber (Utilities|Array|Get(acopy) (Variables|Default|GetTapes%20ID_Copy) Tape_ID)))) true true "(R=1.000000,G=0.133474,B=0.526026,A=1.000000)" 1e+01)
  (Utilities|Array|SetArrayElem (Variables|Default|GetTapes_Possessed) Tape_ID (Utilities|Array|Get(acopy) (Variables|Default|GetTapes%20ID_Copy) Tape_ID) true)
  ;[1 1 1] Print - Liste tapes acquired
  (for _index (range 0 (Utilities|Array|Length (Variables|Default|GetTapes%20ID_Copy)))
    (Development|PrintString (Utilities|String|Append "VHS Possessed" (Utilities|String|ToString(Integer) (.pagenumber (Utilities|Array|Get(acopy) (Variables|Default|GetTapes_Possessed) _index))) "  -  " (Utilities|String|ToString(Name) "None")) true true "(R=0.110418,G=0.458333,B=0.021987,A=1.000000)" 13.0)))

(event EventBeginPlay)

(fn ConstructionScript)

(fn LoopBas
  (if (<= (Variables|Default|GetPageSelection) -1)
    (Variables|Default|SetPageSelection (Utilities|Array|Length (Variables|Default|GetTapes_Possessed)))))

(fn LoopHaut
  (if (> (Variables|Default|GetPageSelection) (Utilities|Array|Length (Variables|Default|GetTapes_Possessed)))
    (Variables|Default|SetPageSelection 0)))