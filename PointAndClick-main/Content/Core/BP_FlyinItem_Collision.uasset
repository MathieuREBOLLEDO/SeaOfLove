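; BP_FlyinItem_Collision is a floating item actor whose mesh bobs vertically and spins continuously.
; The construction script sets its mesh and scale, and swaps in an override material when IsBug is set.
; On BeginPlay, a timeline starts at a random time to desynchronize instances.
; Each update offsets world height from the starting location and adds local rotation, blending yaw speed with a noise track.
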(event EventBeginPlay
  (bind _cube (Variables|Default|GetCube))
  (Variables|Default|SetInitialLocation (Transformation|GetWorldLocation _cube))
  (Variables|Default|SetInitialRotation (Transformation|GetWorldRotation _cube))
  (Variables|Default|SetStartMoment (Math|Random|RandomFloatinRange 0.0 5.0))
  (Utilities|FlowControl|Sequence
    (:then_0
      (bind (_direction _temps _hauteur _rotanoise) (Timeline|Timeline_0 SetNewTime)
        (:Update
          (Transformation|SetWorldLocation (Variables|Default|GetCube) (Math|Vector|Lerp(Vector) (Variables|Default|GetInitialLocation) (Math|Vector|MakeVector (.x (Variables|Default|GetInitialLocation)) (.y (Variables|Default|GetInitialLocation)) (+ (.z (Variables|Default|GetInitialLocation)) _hauteur)) _temps) false false)
          (Transformation|AddLocalRotation (Variables|Default|GetCube) (Math|Rotator|MakeRotator (Variables|Default|GetRotaXSpeed) (Variables|Default|GetRotaYSpeed) (Math|Float|Lerp (Variables|Default|GetRotaZSpeed) _rotanoise _temps)) false false))))
    (:then_1
      (Timeline|Timeline_0 Play))))

(event EventTick
  (params (DeltaSeconds :type Float%20%28single-precision%29)))

(fn ConstructionScript
  (bind _cube (Variables|Default|GetCube))
  (Components|StaticMesh|SetStaticMesh _cube (Variables|Default|GetStaticMeshList_0))
  (Transformation|SetWorldTransform _cube (Math|Transform|MakeTransform (Transformation|GetWorldLocation _cube) (Transformation|GetWorldRotation _cube) (Variables|Default|GetScale)) false false)
  (if (Variables|Default|GetIsBug)
    (Rendering|Material|SetMaterial (Variables|Default|GetCube) 0 (Variables|Default|GetMaterial))))