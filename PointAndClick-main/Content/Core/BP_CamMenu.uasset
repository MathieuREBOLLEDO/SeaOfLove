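; BP_CamMenu is the main menu camera, slowly rotating on a spring arm until play is triggered.
; TransitionCam stops the Tick-driven spin and plays a timeline that eases the arm's rotation and length into a close-up.
; Late in that move, a second timeline ramps up vignette and film grain on the camera's post process, then opens P_EnvMap with game-only input and a hidden cursor.
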(event Custom|TransitionCam
  (bind _returnvalue (Game|GetPlayerController 0))
  (bind _springarm (Variables|Default|GetSpringArm))
  (bind _springarm_2 (Variables|Default|GetSpringArm))
  (Variables|Default|SetIsPressPlay true)
  (Development|PrintString "PLAYYYY")
  (bind _newtrack_0 (Timeline|CamTransition Play)
    (:Update
      (Transformation|SetRelativeRotation _springarm (Math|Rotator|Lerp(Rotator) (Variables|/Script/Engine.SceneComponent|GetRelativeRotation _springarm) "0.000000,270.000000, 0" _newtrack_0 true) false false)
      (Variables|/Script/Engine.SpringArmComponent|SetTargetArmLength _springarm_2 (Math|Float|Lerp (Variables|/Script/Engine.SpringArmComponent|GetTargetArmLength _springarm_2) 7e+01 _newtrack_0))
      (if (> _newtrack_0 0.7)
        (Utilities|FlowControl|DoOnce false
          (:Completed
            (bind _newtrack_0_2 (Timeline|Timeline_0 Play)
              (:Update
                (Variables|/Script/Engine.CameraComponent|SetPostProcessSettings (Variables|Default|GetCameraTurn) (Utilities|Struct|MakePostProcessSettings 0.0 (Math|Float|Lerp 0.0 1e+01 _newtrack_0_2) (Math|Float|Lerp 0.0 1e+02 _newtrack_0_2) (Math|Float|Lerp 0.0 2e+02 _newtrack_0_2))))
              (:Finished
                (Game|OpenLevel(byName) "P_EnvMap")
                (Input|SetInputModeGameOnly _returnvalue)
                (Variables|/Script/Engine.PlayerController|SetbShowMouseCursor _returnvalue false)))))))))

(event EventBeginPlay)

(event Collision|EventActorBeginOverlap
  (params (OtherActor :type Actor%20Object%20Reference)))

(event EventTick
  (params (DeltaSeconds :type Float%20%28single-precision%29))
  (if (not (Variables|Default|GetIsPressPlay))
    (Utilities|FlowControl|Delay 0.05)
    (Transformation|AddLocalRotation (Variables|Default|GetSpringArm) (Math|Rotator|MakeRotator 0.0 0.0 (+ (Variables|Default|GetDelta%20Rotation%20Z%20%28Yaw%29) 0.1)) false false)
    (Input|EnableInput (Game|GetPlayerController 0))))

(fn ConstructionScript)