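; BP_WallColor is an actor that recolors every StaticMeshActor tagged "Wall" to match the currently visible streaming level.
; ChangeWallcolor applies M_Glow when its parameter is 1; otherwise it creates MI_Office_Walls dynamic instances, tinted with the WallColor from the DT_Tapes row whose level is visible.
; The construction script repeats this logic, but picks glow by array index and tints with its Value variable.
; CallSetWallColor is an empty stub.
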(event Custom|Change%20Wall%20color
  (params (NewParam :type Integer))
  (bind _outactors (Actor|GetAllActorsOfClass "/Script/Engine.StaticMeshActor"))
  (for _array_element _outactors
    (if (Actor|ActorHasTag _array_element "Wall")
      (if (== NewParam 1)
        (Rendering|Material|CreateDynamicMaterialInstance (Variables|/Script/Engine.StaticMeshActor|GetStaticMeshComponent _array_element) 0 "/Game/DetectiveStart/Assets/Materials/M_Glow.M_Glow" "None" :!class /Script/Engine.PrimitiveComponent)
        (else
          (bind _returnvalue (Rendering|Material|CreateDynamicMaterialInstance (Variables|/Script/Engine.StaticMeshActor|GetStaticMeshComponent _array_element) 0 "/Game/DetectiveStart/Assets/Materials/Structure/MI_Office_Walls.MI_Office_Walls" "None" :!class /Script/Engine.PrimitiveComponent))
          (bind _outrownames (DataTable|GetDataTableRowNames "/Game/Core/TestAxel/DT_Tapes.DT_Tapes"))
          (for _array_element_2 _outrownames
            (bind _returnvalue_2 (Utilities|GetDataTableRow "/Game/Core/TestAxel/DT_Tapes.DT_Tapes" _array_element_2)
              (:then
                (Utilities|IsValid (Class|GameplayStatics|GetStreamingLevel (.levelname _returnvalue_2))
                  (:Is%20Valid
                    (if (Class|LevelStreaming|IsLevelVisible (Class|GameplayStatics|GetStreamingLevel (.levelname _returnvalue_2)))
                      (Rendering|Material|SetVectorParameterValue _returnvalue "Param" (.wallcolor _returnvalue_2) :!class /Script/Engine.MaterialInstanceDynamic))))))))))))

(event EventBeginPlay)

(event Collision|EventActorBeginOverlap
  (params (OtherActor :type Actor%20Object%20Reference)))

(event EventTick
  (params (DeltaSeconds :type Float%20%28single-precision%29)))

(fn ConstructionScript
  (bind _outactors (Actor|GetAllActorsOfClass "/Script/Engine.StaticMeshActor"))
  (for (_array_element _array_index) _outactors
    (if (Actor|ActorHasTag _array_element "Wall")
      (if (== _array_index 1)
        (Rendering|Material|CreateDynamicMaterialInstance (Variables|/Script/Engine.StaticMeshActor|GetStaticMeshComponent _array_element) 0 "/Game/DetectiveStart/Assets/Materials/M_Glow.M_Glow" "None" :!class /Script/Engine.PrimitiveComponent)
        (else
          (bind _returnvalue (Rendering|Material|CreateDynamicMaterialInstance (Variables|/Script/Engine.StaticMeshActor|GetStaticMeshComponent _array_element) 0 "/Game/DetectiveStart/Assets/Materials/Structure/MI_Office_Walls.MI_Office_Walls" "None" :!class /Script/Engine.PrimitiveComponent))
          (bind _outrownames (DataTable|GetDataTableRowNames "/Game/Core/TestAxel/DT_Tapes.DT_Tapes"))
          (for (_array_element_2 _array_index_2) _outrownames
            (bind _returnvalue_2 (Utilities|GetDataTableRow "/Game/Core/TestAxel/DT_Tapes.DT_Tapes" _array_element_2)
              (:then
                (Utilities|IsValid (Class|GameplayStatics|GetStreamingLevel (.levelname _returnvalue_2))
                  (:Is%20Valid
                    (if (Class|LevelStreaming|IsLevelVisible (Class|GameplayStatics|GetStreamingLevel (.levelname _returnvalue_2)))
                      (if (not (== _array_index_2 1))
                        (Rendering|Material|SetVectorParameterValue _returnvalue "Param" (Variables|Default|GetValue) :!class /Script/Engine.MaterialInstanceDynamic)))))))))))))

(fn CallSetWallColor)